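; Chess piece actor that stores its type, color and square index on an 8x8 board and computes candidate moves.
; InitializePiece sets that state and picks the matching mesh and color material.
; GetValidMoves dispatches by type to index-offset or ray-walking functions, with Queen uniting Rook and Bishop results.
; Moves ignore occupancy and captures, accumulate in an uncleared Moves set, and sliding rays include the current square.
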(event EventBeginPlay)

(event Collision|EventActorBeginOverlap
  (params (OtherActor :type Actor%20Object%20Reference)))

(event EventTick
  (params (DeltaSeconds :type Float%20%28single-precision%29)))

(fn ConstructionScript)

(fn GetValidMoves
  (switch Utilities|FlowControl|Switch|SwitchonPieces (Variables|Default|GetPiece%20Type)
    (:NewEnumerator6
      (return 0))
    (:NewEnumerator0
      (bind _possible_moves (CallFunction|PawnMoves))
      (return _possible_moves))
    (:NewEnumerator1
      (bind _moves1 (CallFunction|RookMoves))
      (return _moves1))
    (:NewEnumerator2
      (bind _newparam (CallFunction|KnightMoves))
      (return _newparam))
    (:NewEnumerator3
      (bind _newparam_2 (CallFunction|BishopMoves))
      (return _newparam_2))
    (:NewEnumerator4
      (bind _newparam_3 (CallFunction|QueenMoves))
      (return _newparam_3))
    (:NewEnumerator5
      (bind _newparam_4 (CallFunction|KingMoves))
      (return _newparam_4))))

(fn PawnMoves
  (bind (_row _column) (Utilities|GetRow/ColLocation))
  (bind _row_2 (Utilities|GetRow/ColLocation))
  (bind _location (Variables|Default|GetLocation))
  (bind _location_2 (Variables|Default|GetLocation))
  (if (or (== _row 0) (== _column 7)) ; Has pawn reached the end?
    (return 0)
    (else
      (if (Variables|Default|GetIsWhite) ; Is pawn black or white?
        (Utilities|Set|Add (LocalVariables|GetMoves) (+ _location_2 8))
        ;[1 1 1] Has pawn not moved yet?
        (if (== _row_2 1)
          (Utilities|Set|Add (LocalVariables|GetMoves) (+ _location 16)))
        (else
          (Utilities|Set|Add (LocalVariables|GetMoves) (+ _location_2 -8))
          (if (== _row_2 6)
            (Utilities|Set|Add (LocalVariables|GetMoves) (+ _location -16)))))
      (return (LocalVariables|GetMoves)))))

(fn RookMoves
  (bind (_row _column) (Utilities|GetRow/ColLocation))
  (bind (_row_2 _column_2) (Utilities|GetRow/ColLocation))
  (bind (_row_3 _column_3) (Utilities|GetRow/ColLocation))
  (bind (_row_4 _column_4) (Utilities|GetRow/ColLocation))
  (Utilities|FlowControl|Sequence ; Possible positions starting from 12 o'clock clockwise
    (:then_0
      (bind _output_get (LocalVariables|SetCurrent%20Row _row_2))
      (while (Utilities|OnBoard? _output_get _column_2)
        (Utilities|Set|Add (LocalVariables|GetMoves) (Utilities|Row/ColtoLocation _output_get _column_2))
        (LocalVariables|SetCurrent%20Row (+ (LocalVariables|GetCurrent%20Row) 1))))
    (:then_1
      (bind _output_get_2 (LocalVariables|SetCurrent%20Column _column_3))
      (while (Utilities|OnBoard? _row_3 _output_get_2)
        (Utilities|Set|Add (LocalVariables|GetMoves) (Utilities|Row/ColtoLocation _row_3 _output_get_2))
        (LocalVariables|SetCurrent%20Column (+ 1 (LocalVariables|GetCurrent%20Column)))))
    (:then_2
      (bind _output_get_3 (LocalVariables|SetCurrent%20Row _row_4))
      (while (Utilities|OnBoard? _output_get_3 _column_4)
        (Utilities|Set|Add (LocalVariables|GetMoves) (Utilities|Row/ColtoLocation _output_get_3 _column_4))
        (LocalVariables|SetCurrent%20Row (+ (LocalVariables|GetCurrent%20Row) -1))))
    (:then_3
      (bind _output_get_4 (LocalVariables|SetCurrent%20Column _column))
      (while (Utilities|OnBoard? _row _output_get_4)
        (Utilities|Set|Add (LocalVariables|GetMoves) (Utilities|Row/ColtoLocation _row _output_get_4))
        (LocalVariables|SetCurrent%20Column (+ -1 (LocalVariables|GetCurrent%20Column)))))
    (:then_4
      (return (LocalVariables|GetMoves)))))

(fn KnightMoves
  (bind (_row _column) (Utilities|GetRow/ColLocation))
  (bind (_row_2 _column_2) (Utilities|GetRow/ColLocation))
  (bind (_row_3 _column_3) (Utilities|GetRow/ColLocation))
  (bind (_row_4 _column_4) (Utilities|GetRow/ColLocation))
  (bind (_row_5 _column_5) (Utilities|GetRow/ColLocation))
  (bind (_row_6 _column_6) (Utilities|GetRow/ColLocation))
  (bind (_row_7 _column_7) (Utilities|GetRow/ColLocation))
  (bind (_row_8 _column_8) (Utilities|GetRow/ColLocation))
  (bind _moves (LocalVariables|GetMoves))
  (Utilities|FlowControl|Sequence ; Possible positions starting from 12 o'clock clockwise
    (:then_0
      (if (and (<= _row_2 5) (<= _column_2 6))
        (Utilities|Set|Add _moves (+ (Variables|Default|GetLocation) 17))))
    (:then_1
      (if (and (<= _row_3 6) (<= _column_3 5))
        (Utilities|Set|Add _moves (+ (Variables|Default|GetLocation) 10))))
    (:then_2
      (if (and (>= _row_4 1) (<= _column_4 5))
        (Utilities|Set|Add _moves (+ (Variables|Default|GetLocation) -6))))
    (:then_3
      (if (and (>= _row_5 2) (<= _column_5 6))
        (Utilities|Set|Add _moves (+ (Variables|Default|GetLocation) -15))))
    (:then_4
      (if (and (>= _row_6 2) (>= _column_6 1))
        (Utilities|Set|Add _moves (+ (Variables|Default|GetLocation) -17))))
    (:then_5
      (if (and (>= _row_7 1) (>= _column_7 2))
        (Utilities|Set|Add _moves (+ (Variables|Default|GetLocation) -10))))
    (:then_6
      (if (and (<= _row_8 6) (>= _column_8 2))
        (Utilities|Set|Add _moves (+ (Variables|Default|GetLocation) 6))))
    (:then_7
      (if (and (<= _row 5) (>= _column 1))
        (Utilities|Set|Add _moves (+ (Variables|Default|GetLocation) 15))))
    (:then_8
      (return (LocalVariables|GetMoves)))))

(fn BishopMoves
  (bind (_row _column) (Utilities|GetRow/ColLocation))
  (bind (_row_2 _column_2) (Utilities|GetRow/ColLocation))
  (bind (_row_3 _column_3) (Utilities|GetRow/ColLocation))
  (bind (_row_4 _column_4) (Utilities|GetRow/ColLocation))
  (Utilities|FlowControl|Sequence ; Possible positions starting from 12 o'clock clockwise
    (:then_0
      (bind _output_get (LocalVariables|SetCurrent%20Row _row_4))
      (bind _output_get_2 (LocalVariables|SetCurrent%20Column _column_4))
      (while (Utilities|OnBoard? _output_get _output_get_2)
        (Utilities|Set|Add (LocalVariables|GetMoves) (Utilities|Row/ColtoLocation _output_get _output_get_2))
        (LocalVariables|SetCurrent%20Row (+ (LocalVariables|GetCurrent%20Row) 1))
        (LocalVariables|SetCurrent%20Column (+ (LocalVariables|GetCurrent%20Column) 1))))
    (:then_1
      (bind _output_get_3 (LocalVariables|SetCurrent%20Row _row_2))
      (bind _output_get_4 (LocalVariables|SetCurrent%20Column _column_2))
      (while (Utilities|OnBoard? _output_get_3 _output_get_4)
        (Utilities|Set|Add (LocalVariables|GetMoves) (Utilities|Row/ColtoLocation _output_get_3 _output_get_4))
        (LocalVariables|SetCurrent%20Row (+ (LocalVariables|GetCurrent%20Row) -1))
        (LocalVariables|SetCurrent%20Column (+ (LocalVariables|GetCurrent%20Column) 1))))
    (:then_2
      (bind _output_get_5 (LocalVariables|SetCurrent%20Row _row_3))
      (bind _output_get_6 (LocalVariables|SetCurrent%20Column _column_3))
      (while (Utilities|OnBoard? _output_get_5 _output_get_6)
        (Utilities|Set|Add (LocalVariables|GetMoves) (Utilities|Row/ColtoLocation _output_get_5 _output_get_6))
        (LocalVariables|SetCurrent%20Row (+ (LocalVariables|GetCurrent%20Row) -1))
        (LocalVariables|SetCurrent%20Column (+ (LocalVariables|GetCurrent%20Column) -1))))
    (:then_3
      (bind _output_get_7 (LocalVariables|SetCurrent%20Row _row))
      (bind _output_get_8 (LocalVariables|SetCurrent%20Column _column))
      (while (Utilities|OnBoard? _output_get_7 _output_get_8)
        (Utilities|Set|Add (LocalVariables|GetMoves) (Utilities|Row/ColtoLocation _output_get_7 _output_get_8))
        (LocalVariables|SetCurrent%20Row (+ (LocalVariables|GetCurrent%20Row) 1))
        (LocalVariables|SetCurrent%20Column (+ (LocalVariables|GetCurrent%20Column) -1))))
    (:then_4
      (return (LocalVariables|GetMoves)))))

(fn QueenMoves
  (bind _moves1 (CallFunction|RookMoves))
  (bind _newparam (CallFunction|BishopMoves))
  (bind _result (Utilities|Set|Union _newparam _moves1))
  (return _result))

(fn KingMoves
  (bind _row (Utilities|GetRow/ColLocation))
  (bind _column (Utilities|GetRow/ColLocation))
  (bind _row_2 (Utilities|GetRow/ColLocation))
  (bind _column_2 (Utilities|GetRow/ColLocation))
  (bind _moves (LocalVariables|GetMoves))
  (bind _returnvalue (<= _row 6))
  (bind _returnvalue_2 (<= _column 6))
  (bind _returnvalue_3 (>= _row_2 1))
  (bind _returnvalue_4 (>= _column_2 1))
  (Utilities|FlowControl|Sequence ; Possible positions starting from 12 o'clock clockwise
    (:then_0
      (if _returnvalue
        (Utilities|Set|Add _moves (+ (Variables|Default|GetLocation) 8))))
    (:then_1
      (if (and _returnvalue _returnvalue_2)
        (Utilities|Set|Add _moves (+ (Variables|Default|GetLocation) 9))))
    (:then_2
      (if _returnvalue_2
        (Utilities|Set|Add _moves (+ (Variables|Default|GetLocation) 1))))
    (:then_3
      (if (and _returnvalue_2 _returnvalue_3)
        (Utilities|Set|Add _moves (+ (Variables|Default|GetLocation) -7))))
    (:then_4
      (if _returnvalue_3
        (Utilities|Set|Add _moves (+ (Variables|Default|GetLocation) -8))))
    (:then_5
      (if (and _returnvalue_3 _returnvalue_4)
        (Utilities|Set|Add _moves (+ (Variables|Default|GetLocation) -9))))
    (:then_6
      (if _returnvalue_4
        (Utilities|Set|Add _moves (+ (Variables|Default|GetLocation) -1))))
    (:then_7
      (if (and _returnvalue_4 _returnvalue)
        (Utilities|Set|Add _moves (+ (Variables|Default|GetLocation) 7))))
    (:then_8
      (return (LocalVariables|GetMoves)))))

(fn InitializePiece
  (params (Location :type Integer) (Type :type Pieces%20Enum :default "NewEnumerator6") (Is%20White? :type Boolean))
  (bind (_pawn _rook _knight _bishop _queen _king) (|GetMeshes_2))
  (bind _piece_colors (Variables|Default|GetPiece%20Colors))
  (bind _piece_mesh (Variables|Default|GetPiece%20Mesh))
  (Variables|Default|SetLocation Location)
  (bind _output_get (Variables|Default|SetPiece%20Type Type))
  (Variables|Default|SetIsWhite Is%20White?)
  ;[1 1 1] Set Piece's Mesh Depending on Type
  (switch Utilities|FlowControl|Switch|SwitchonPieces _output_get
    (:NewEnumerator0
      (Components|StaticMesh|SetStaticMesh _piece_mesh _pawn))
    (:NewEnumerator1
      (Components|StaticMesh|SetStaticMesh _piece_mesh _rook))
    (:NewEnumerator2
      (Components|StaticMesh|SetStaticMesh _piece_mesh _knight))
    (:NewEnumerator3
      (Components|StaticMesh|SetStaticMesh _piece_mesh _bishop))
    (:NewEnumerator4
      (Components|StaticMesh|SetStaticMesh _piece_mesh _queen))
    (:NewEnumerator5
      (Components|StaticMesh|SetStaticMesh _piece_mesh _king)))
  ;[1 1 1] Set Piece's Color
  (if (Variables|Default|GetIsWhite)
    (Rendering|Material|SetMaterial (Variables|Default|GetPiece%20Mesh) 0 (Utilities|Array|Get(acopy) _piece_colors))
    (else
      (Rendering|Material|SetMaterial (Variables|Default|GetPiece%20Mesh) 0 (Utilities|Array|Get(acopy) _piece_colors 1)))))